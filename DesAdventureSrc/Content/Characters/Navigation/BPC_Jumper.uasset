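; Character component in the navigation folder that launches its owning Character along a ballistic arc to a destination through JumpTo.
; Height is measured from the capsule bottom, and vertical speed is derived from gravity and that rise plus extra clearance, capped at the movement component's JumpZVelocity.
; A quadratic flight-time solution then sets horizontal speed, and LaunchCharacter overrides the current velocity with the result.
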(event EventBeginPlay
  (bind _ascharacter (Utilities|Casting|CastToCharacter (Components|GetOwner)))
  (Variables|Default|SetOwningCharacter _ascharacter))

(fn CalculateJumpVector
  (params (Destination :type Vector))
  (bind _owningcharacter (Variables|Default|GetOwningCharacter))
  (bind _returnvalue (Transformation|GetActorLocation _owningcharacter))
  (return (Math|Vector|MakeVector (- (.x Destination) (.x _returnvalue)) (- (.y Destination) (.y _returnvalue)) (|(zdest-(zact-halfheight)) (.z Destination) (.z _returnvalue) (Components|Capsule|GetScaledCapsuleHalfHeight (Variables|/Script/Engine.Character|GetCapsuleComponent _owningcharacter))))))

(fn CalculateJumpVelocity
  (params (JumpVector :type Vector))
  (bind _force (CallFunction|CalculateRequiredPossibleJumpForce (.z JumpVector)))
  (bind _time (CallFunction|CalculateJumpTime (.z JumpVector) _force))
  (return (Math|Vector|MakeVector (/ (.x JumpVector) _time) (/ (.y JumpVector) _time) _force)))

(fn CalculateJumpTime
  (params (Z :type Float%20%28double-precision%29) (VelZ :type Float%20%28double-precision%29))
  (return (|((vz+(sqrt(((vz*vz)-((2*(abs(g)))*z)))))/(abs(g))) (Components|Movement|GetGravityZ (Variables|/Script/Engine.Character|GetCharacterMovement (Variables|Default|GetOwningCharacter))) VelZ Z)))

(fn CalculateRequiredPossibleJumpForce
  (params (Z :type Float%20%28double-precision%29))
  (bind _owningcharacter (Variables|Default|GetOwningCharacter))
  (bind _charactermovement (Variables|/Script/Engine.Character|GetCharacterMovement _owningcharacter))
  (return (Math|Float|Min(Float) (Variables|/Script/Engine.CharacterMovementComponent|GetJumpZVelocity _charactermovement) (|(sqrt(((((2*z)*g)*g)/((2*(abs(g)))-1)))) (Components|Movement|GetGravityZ _charactermovement) (|((max(z,0))+{1D1227ED-64CA-4B4C-8997-25F9A131AB41}) Z)))))

(fn Jumpto
  (params (Destination :type Vector))
  (bind _jumpvec (CallFunction|CalculateJumpVector Destination))
  (bind _jumpvelocity (CallFunction|CalculateJumpVelocity _jumpvec))
  (Character|LaunchCharacter (Variables|Default|GetOwningCharacter) _jumpvelocity true true))