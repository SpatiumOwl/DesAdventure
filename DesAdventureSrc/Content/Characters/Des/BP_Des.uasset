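; BP_Des is the player character Des, with health shown on the game mode's UI, team identity, and death that halts movement.
; Its construction script passes range settings to slash, absorb and dive components.
; Each tick, a downward launch shortens jumps when the controller's jump flag is off during ascent.
; A forward sphere trace also finds interactable actors each tick, toggling the UI prompt and swapping Enhanced Input mapping contexts.
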(event `InitializePlayer`
  ;[1 1 1] Get controller
  (bind _aspc_des (cast `/Game/Characters/Des/PC_Des` (`self.GetController`)))
  (set `self.PlayerController` _aspc_des)
  ;[1 1 1] Restore health
  (bind _output_get (set `self.CurrentHealth` (`self.MaxHealth`)))
  (`/Game/UI/WB_PlayerUI.UpdateHealthUI` (`self.PlayerUI`) _output_get (`self.MaxHealth`)))

(event `self.ReceiveBeginPlay`
  ;[1 1 1] Set up UI
  (bind _asgm_des (cast `/Game/Characters/Des/GM_Des` (`GameplayStatics.GetGameMode`)))
  (set `self.PlayerUI` (`/Game/Characters/Des/GM_Des.PlayerUI` _asgm_des))
  ;[1 1 1] Set up player
  (`self.InitializePlayer`))

(event `self.ReceiveTick`
  (params (DeltaSeconds :type "Float (single-precision)"))
  ;[1 1 1] Jump Fix
  (`self.JumpFix` DeltaSeconds)
  (`self.InteractCheck`))

(event `self.ReceiveAnyDamage`
  (params (Damage :type "Float (single-precision)") (DamageType :type "DamageType Object Reference") (InstigatedBy :type "Controller Object Reference") (DamageCauser :type "Actor Object Reference"))
  ;[1 1 1] Receive Damage
  (if (not (`self.bDeath`))
    (bind _output_get (set `self.CurrentHealth` (`KismetMathLibrary.FClamp` (- (`self.CurrentHealth`) Damage) 0.0 (`self.MaxHealth`))))
    (`/Game/UI/WB_PlayerUI.UpdateHealthUI` (`self.PlayerUI`) _output_get (`self.MaxHealth`))
    (if (== (`self.CurrentHealth`) 0.0)
      (`self.Death`))))

(event `Death`
  (bind _charactermovement (`self.CharacterMovement`))
  ;[1 1 1] Die
  (set `self.bDeath` false)
  (`MovementComponent.StopMovementImmediately` _charactermovement)
  (`CharacterMovementComponent.DisableMovement` _charactermovement))

(fn `InteractCheck`
  (returns (Actor :type "Actor Object Reference"))
  (locals (InteractActor :type "Actor Object Reference") (InteractDistance :type "Float (single-precision)" :default 120.0) (InteractRadius :type "Float (single-precision)" :default 80.0))
  (bind _returnvalue (`self.K2_GetActorLocation`))
  (bind _playerui (`self.PlayerUI`))
  (bind _returnvalue_2 (pcsubsystem `EnhancedInputLocalPlayerSubsystem` (`self.PlayerController`)))
  (bind _returnvalue_3 (pcsubsystem `EnhancedInputLocalPlayerSubsystem` (`self.PlayerController`)))
  (bind _outhit (`KismetSystemLibrary.SphereTraceSingle` _returnvalue (+ _returnvalue (* (`KismetMathLibrary.GetForwardVector` (`self.K2_GetActorRotation`)) (`local.InteractDistance`))) (`local.InteractRadius`) "TraceTypeQuery2"))
  (if (`GameplayStatics.BreakHitResult` _outhit)
    (if (`KismetSystemLibrary.DoesImplementInterface` (`.HitActor` (`GameplayStatics.BreakHitResult` _outhit)) "/Game/Characters/NPCs/BPI_Interactable.BPI_Interactable_C")
      (bind _output_get (set `local.InteractActor` (`.HitActor` (`GameplayStatics.BreakHitResult` _outhit))))
      (`/Game/UI/WB_PlayerUI.DisplayMessage` _playerui _output_get true)
      (`EnhancedInputSubsystemInterface.RemoveMappingContext` _returnvalue_3 "/Game/Input/IMC_DesRegular.IMC_DesRegular" (struct))
      (`EnhancedInputSubsystemInterface.AddMappingContext` _returnvalue_3 "/Game/Input/IMC_DesInteractable.IMC_DesInteractable" 0 (struct))
      (else
        (`/Game/UI/WB_PlayerUI.DisplayMessage` _playerui null false :!label _label)
        (`EnhancedInputSubsystemInterface.RemoveMappingContext` _returnvalue_2 "/Game/Input/IMC_DesInteractable.IMC_DesInteractable" (struct))
        (`EnhancedInputSubsystemInterface.AddMappingContext` _returnvalue_2 "/Game/Input/IMC_DesRegular.IMC_DesRegular" 0 (struct))))
    (else
      (goto _label)))
  (return (`local.InteractActor`)))

(fn `JumpFix`
  (params (DeltaSeconds :type "Float (double-precision)" :default 1.0))
  (bind (_returnvalue_x _returnvalue_y _returnvalue_z) (`KismetMathLibrary.BreakVector` (`self.GetVelocity`)))
  (if (and (> _returnvalue_z 0.05) (not (`/Game/Characters/Des/PC_Des.IsJumping` (`self.PlayerController`))))
    ;[1 1 1] Diminishing jump
    (`self.LaunchCharacter` (`KismetMathLibrary.MakeVector` 0.0 0.0 (* (* DeltaSeconds (`self.LowJumpForce`)) -1.0)))))

(fn `UserConstructionScript`
  (`KismetArrayLibrary.Array_Append` (`/Game/Characters/Des/Actions/BPC_Slash.Range` (`self.BPC_Slash`)) (`|MakeArray` (`self.Slash Range`) (`self.Slash Range_ext`)))
  (`KismetArrayLibrary.Array_Append` (`/Game/Characters/Des/Actions/BPC_Absorb.Range` (`self.BPC_Absorb`)) (`|MakeArray` (`self.Slash Range`) (`self.Slash Range_ext`)))
  (set `/Game/Characters/Des/Actions/BPC_Dive.Range` (`self.DiveRange`) (`self.BPC_Dive`)))

(fn `Which Team`
  (returns (Team :type "/Game/Characters/Enum_Teams Enum"))
  (return "NewEnumerator0"))