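; Actor component for Des's absorb ability, which drains health from nearby angered enemies to heal the owning character.
; Absorb gathers unique characters overlapping the Range components, then damages opposing-team members whose BPC_Angryable is angry by that component's AbsorbDamage.
; Each hit reports an AI damage event and heals the owner by a fraction through negative damage.
; A Tick timer limits chained uses, locking Absorb at MaxSequence until the cooldown expires.
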(event `self.ReceiveBeginPlay`
  ;[1 1 1] Initialize
  (bind _ascharacter (cast `Character` (`self.GetOwner`)))
  (bind _output_get (set `self.OwnerPawn` _ascharacter))
  (bind _asplayer_controller (cast `PlayerController` (`Pawn.GetController` _output_get)))
  (set `self.OwnerController` _asplayer_controller))

(event `Absorb`
  ;[1 1 1] Slash
  (if (not (`self.IsOnCooldown`))
    (`KismetSystemLibrary.PrintString` "ABSORB!" true true (struct :`R` 0.450652 :`B` 1.0 :`A` 1.0))
    (`self.PerformAbsorb`)
    (`/Engine/EditorBlueprintResources/StandardMacros.IncrementInt` (`self.CurrentSequenceLength`)
      (:`  `
        (set `self.TimeUntilCooldown` (`self.TotalCooldownTime`))
        (if (== (`self.CurrentSequenceLength`) (`self.MaxSequence`))
          (set `self.IsOnCooldown` true))))))

(event `self.ReceiveTick`
  (params (DeltaSeconds :type "Float (single-precision)"))
  ;[1 1 1] Cooldown
  (bind _output_get (set `self.TimeUntilCooldown` (- (`self.TimeUntilCooldown`) DeltaSeconds)))
  (if (<= _output_get 0.0)
    (set `self.IsOnCooldown` false)
    (set `self.CurrentSequenceLength` 0)))

(fn `PerformAbsorb`
  (bind _ownerpawn (`self.OwnerPawn`))
  (bind _returnvalue (`Actor.GetComponentByClass` (`self.CurrentEnemy`) "/Game/Characters/Enemies/BPC_Angryable.BPC_Angryable_C"))
  ;[1 1 1] Absorb
  ;;[1 1 1] Make list of characters who got into the range
  (set `self.OverlappingCharacters` (`|MakeSet` null :!type "Actor Object Reference"))
  (for _array_element (`self.Range`)
    (`BlueprintSetLibrary.Set_AddItems` (`self.OverlappingCharacters`) (`PrimitiveComponent.GetOverlappingActors` _array_element "/Script/Engine.Character")))
  (bind _result (`BlueprintSetLibrary.Set_ToArray` (`self.OverlappingCharacters`)))
  (for _array_element_2 _result
    ;;[1 1 1] Check if an enemy
    (bind _asbpi_teamable (cast `/Game/Characters/BPI_Teamable` _array_element_2))
    (bind _team (`/Game/Characters/BPI_Teamable.Which Team` _asbpi_teamable))
    (if (`|EnumEquality` _team "NewEnumerator1")
      (set `self.CurrentEnemy` _array_element_2)
      ;;[1 1 1] Apply if angered
      (if (`KismetSystemLibrary.IsValid` _returnvalue)
        (set `self.CurrentAngeryable` _returnvalue)
        (bind _result_2 (`/Game/Characters/Enemies/BPC_Angryable.Is Angry` (`self.CurrentAngeryable`)))
        (if _result_2
          (bind _returnvalue_2 (`GameplayStatics.ApplyDamage` (`self.CurrentEnemy`) (`/Game/Characters/Enemies/BPC_Angryable.AbsorbDamage` (`self.CurrentAngeryable`)) (`self.OwnerController`) null "/Game/DamageTypes/DT_Absorption.DT_Absorption_C"))
          (`AISense_Damage.ReportDamageEvent` (`self.CurrentEnemy`) _ownerpawn _returnvalue_2 (`Actor.K2_GetActorLocation` _ownerpawn))
          ;;[1 1 1] Heal character
          (`GameplayStatics.ApplyDamage` (`self.OwnerPawn`) (* (* _returnvalue_2 (`self.RelativeAbsorbedHealth`)) -1.0) (`self.OwnerController`) null "/Game/DamageTypes/DT_Absorption.DT_Absorption_C"))))))