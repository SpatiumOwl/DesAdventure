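; Actor component that gives its owning character a forward dash, limited to one use until the character is no longer falling.
; PerformDash disables movement and player input, ignores Pawn collision and constrains the plane for the dash duration.
; Tick drives DashTick's swept capsule-forward offsets at constant speed and clears the used flag.
; On finish it restores input and walking, but sets capsule object type rather than resetting the Pawn response.
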(event `self.ReceiveBeginPlay`
  ;[1 1 1] Initialize
  (bind _ascharacter (cast `Character` (`self.GetOwner`)))
  (bind _output_get (set `self.OwnerPawn` _ascharacter))
  (bind _asplayer_controller (cast `PlayerController` (`Pawn.GetController` _output_get)))
  (set `self.OwnerController` _asplayer_controller))

(event `Dash`
  ;[1 1 1] Dash
  (if (not (`self.DashUsed`))
    (`self.Perform Dash`)))

(event `Perform Dash`
  (bind _ownercontroller (`self.OwnerController`))
  (bind _ownercontroller_2 (`self.OwnerController`))
  ;[1 1 1] Perform dash
  (`MovementComponent.StopMovementImmediately` (`Character.CharacterMovement` (`self.OwnerPawn`)))
  (`CharacterMovementComponent.DisableMovement` (`Character.CharacterMovement` (`self.OwnerPawn`)))
  (`Actor.DisableInput` _ownercontroller_2 _ownercontroller_2)
  (`PrimitiveComponent.SetCollisionResponseToChannel` (`Character.CapsuleComponent` (`self.OwnerPawn`)) "ECC_Pawn" "ECR_Ignore")
  (`MovementComponent.SetPlaneConstraintNormal` (`Character.CharacterMovement` (`self.OwnerPawn`)) (0.0 0.0 1.0))
  (set `self.IsDashing` true)
  (`KismetSystemLibrary.Delay` (`self.DashDuration`))
  (set `self.IsDashing` false)
  (`PrimitiveComponent.SetCollisionObjectType` (`Character.CapsuleComponent` (`self.OwnerPawn`)) "ECC_Pawn")
  (`MovementComponent.SetPlaneConstraintNormal` (`Character.CharacterMovement` (`self.OwnerPawn`)) (0.0 0.0 0.0))
  (`Actor.EnableInput` _ownercontroller _ownercontroller)
  (`CharacterMovementComponent.SetMovementMode` (`Character.CharacterMovement` (`self.OwnerPawn`)) "MOVE_Walking" 0)
  (set `self.DashUsed` true))

(event `self.ReceiveTick`
  (params (DeltaSeconds :type "Float (single-precision)"))
  ;[1 1 1] Advance character's dash
  (if (`self.IsDashing`)
    (`self.DashTick` DeltaSeconds))
  ;[1 1 1] Restore dash
  (if (`self.DashUsed`)
    (if (not (`NavMovementComponent.IsFalling` (`Character.CharacterMovement` (`self.OwnerPawn`))))
      (set `self.DashUsed` false))))

(fn `DashTick`
  (params (DeltaTime :type "Float (double-precision)"))
  (`Actor.K2_AddActorWorldOffset` (`self.OwnerPawn`) (* DeltaTime (/ (* (`SceneComponent.GetForwardVector` (`Character.CapsuleComponent` (`self.OwnerPawn`))) (`self.DashDistance`)) (`self.DashDuration`))) true false))