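; BPC_Slash is a component that gives its owning character a slash attack with a limited combo and cooldown.
; Each slash gathers overlapping characters from the Range components into a de-duplicated set, then damages those on one specific team via BPI_Teamable.
; Every slash restarts a timer counted down on Tick; reaching the combo limit blocks slashing until it expires, which also resets the combo.
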(event `self.ReceiveBeginPlay`
  ;[1 1 1] Initialize
  (bind _ascharacter (cast `Character` (`self.GetOwner`)))
  (set `self.OwnerController` (`Pawn.GetController` _ascharacter)))

(event `Slash`
  ;[1 1 1] Slash
  (if (not (`self.IsOnCooldown`))
    (`KismetSystemLibrary.PrintString` "SLASH!" true true (struct :`R` 1.0 :`G` 0.036154 :`A` 1.0))
    (`self.PerformOneSlash`)
    (`/Engine/EditorBlueprintResources/StandardMacros.IncrementInt` (`self.CurrentSequenceLength`)
      (:`  `
        (set `self.TimeUntilCooldown` (`self.TotalCooldownTime`))
        (if (== (`self.CurrentSequenceLength`) (`self.MaxSequence`))
          (set `self.IsOnCooldown` true))))))

(event `self.ReceiveTick`
  (params (DeltaSeconds :type "Float (single-precision)"))
  ;[1 1 1] Cooldown
  (bind _output_get (set `self.TimeUntilCooldown` (- (`self.TimeUntilCooldown`) DeltaSeconds)))
  (if (<= _output_get 0.0)
    (set `self.IsOnCooldown` false)
    (set `self.CurrentSequenceLength` 0)))

(fn `PerformOneSlash`
  ;[1 1 1] Slash
  (set `self.OverlappingCharacters` (`|MakeSet` null :!type "Actor Object Reference"))
  (for _array_element (`self.Range`)
    (`BlueprintSetLibrary.Set_AddItems` (`self.OverlappingCharacters`) (`PrimitiveComponent.GetOverlappingActors` _array_element "/Script/Engine.Character")))
  (bind _result (`BlueprintSetLibrary.Set_ToArray` (`self.OverlappingCharacters`)))
  (for _array_element_2 _result
    (bind _asbpi_teamable (cast `/Game/Characters/BPI_Teamable` _array_element_2))
    (bind _team (`/Game/Characters/BPI_Teamable.Which Team` _asbpi_teamable))
    (if (`|EnumEquality` _team "NewEnumerator1")
      (`GameplayStatics.ApplyDamage` _array_element_2 (`self.Damage`) (`self.OwnerController`) null "/Game/DamageTypes/DT_Regular.DT_Regular_C"))))