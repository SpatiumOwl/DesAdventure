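; BPC_Dive is a character component for a ground-slam dive with a cooldown.
; Dive disables input, freezes the character mid-air for a pause, then launches it straight down.
; Tick counts down the cooldown and, only once it has expired, checks for landing.
; Landing damages characters of one team overlapping Range, found through BPI_Teamable, then restores input after a ground pause.
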(event `self.ReceiveBeginPlay`
  ;[1 1 1] Initialize
  (bind _ascharacter (cast `Character` (`self.GetOwner`)))
  (bind _output_get (set `self.OwnerPawn` _ascharacter))
  (bind _asplayer_controller (cast `PlayerController` (`Pawn.GetController` _output_get)))
  (set `self.OwnerController` _asplayer_controller))

(event `Dive`
  ;[1 1 1] Dive
  (if (not (`self.IsOnCooldown`))
    (`KismetSystemLibrary.PrintString` "DIVE!" true true (struct :`R` 1.0 :`G` 0.34678 :`A` 1.0))
    (`self.Perform Dive`)
    (set `self.TimeUntilCooldown` (`self.TotalCooldownTime`))
    (set `self.IsOnCooldown` true)))

(event `self.ReceiveTick`
  (params (DeltaSeconds :type "Float (single-precision)"))
  ;[1 1 1] Cooldown
  (bind _output_get (set `self.TimeUntilCooldown` (- (`self.TimeUntilCooldown`) DeltaSeconds)))
  (if (<= _output_get 0.0)
    (set `self.IsOnCooldown` false)
    ;[1 1 1] Monitor diving
    (if (`self.IsDiving`)
      (if (not (`NavMovementComponent.IsFalling` (`Character.CharacterMovement` (`self.OwnerPawn`))))
        (`self.Finish Dive`)))))

(event `Perform Dive`
  (bind _ownercontroller (`self.OwnerController`))
  (bind _charactermovement (`Character.CharacterMovement` (`self.OwnerPawn`)))
  ;[1 1 1] Perform Dive
  ;;[1 1 1] Pause in the air
  (`Actor.DisableInput` _ownercontroller _ownercontroller)
  (`MovementComponent.SetPlaneConstraintNormal` (`Character.CharacterMovement` (`self.OwnerPawn`)) (0.0 0.0 1.0))
  (`MovementComponent.StopMovementImmediately` _charactermovement)
  (`CharacterMovementComponent.DisableMovement` _charactermovement)
  (`KismetSystemLibrary.Delay` (`self.AirPauseTime`))
  (`CharacterMovementComponent.SetMovementMode` (`Character.CharacterMovement` (`self.OwnerPawn`)) "MOVE_Walking" 0)
  (`MovementComponent.SetPlaneConstraintNormal` (`Character.CharacterMovement` (`self.OwnerPawn`)) (0.0 0.0 0.0))
  ;;[1 1 1] Go Down
  (set `self.IsDiving` true)
  (`Character.LaunchCharacter` (`self.OwnerPawn`) (`KismetMathLibrary.MakeVector` 0.0 0.0 (- 0.0 (`self.LaunchDownPower`))) true true))

(event `Finish Dive`
  (bind _ownercontroller (`self.OwnerController`))
  ;[1 1 1] Finish Dive
  (set `self.IsDiving` false)
  ;;[1 1 1] Damage all enemies
  (for _array_element (`PrimitiveComponent.GetOverlappingActors` (`self.Range`) "/Script/Engine.Character")
    (bind _asbpi_teamable (cast `/Game/Characters/BPI_Teamable` _array_element))
    (bind _team (`/Game/Characters/BPI_Teamable.Which Team` _asbpi_teamable))
    (if (`|EnumEquality` _team "NewEnumerator1")
      (`GameplayStatics.ApplyDamage` _array_element (`self.Damage`) (`self.OwnerController`))))
  ;;[1 1 1] Delay after landing
  (`KismetSystemLibrary.Delay` (`self.GroundPauseTime`))
  (`Actor.EnableInput` _ownercontroller _ownercontroller))