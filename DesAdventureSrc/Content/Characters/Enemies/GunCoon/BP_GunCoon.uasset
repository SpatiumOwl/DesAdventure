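; BP_GunCoon is a gun-wielding enemy character that shoots the player and can jump between platforms.
; Shoot applies GunDamage to every BP_Des overlapping its ShootingRange, then launches the enemy opposite its capsule's forward vector as recoil, scaled by ThrowbackForce.
; On reaching a platform nav link proxy, it hands the destination to its BPC_Jumper component, if present, to perform the jump.
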(event `Shoot`
  (bind _returnvalue (* (`self.ThrowbackForce`) -1.0))
  ;[1 1 1] Shoot the player
  ;;[1 1 1] Shoot the character in the vicinity
  (for _array_element (`PrimitiveComponent.GetOverlappingActors` (`self.Shooting Range`) "/Game/Characters/Des/BP_Des.BP_Des_C")
    (bind _asbp_des (cast `/Game/Characters/Des/BP_Des` _array_element))
    (`/Game/Characters/Des/BP_Des.Receive Damage` _asbp_des (`self.Gun Damage`)))
  ;;[1 1 1] Receive kickback from a shot and get contused
  (`self.LaunchCharacter` (* (`SceneComponent.GetForwardVector` (`self.CapsuleComponent`)) (`KismetMathLibrary.MakeVector` _returnvalue _returnvalue _returnvalue))))

(event `/Game/Characters/Navigation/BPI_PlatformNav.ReachedPlatformNavLinkProxy`
  (params (Destination :type "Vector Structure"))
  (bind _returnvalue (`self.GetComponentByClass` "/Game/Characters/Navigation/BPC_Jumper.BPC_Jumper_C"))
  (if (`KismetSystemLibrary.IsValid` _returnvalue)
    (`/Game/Characters/Navigation/BPC_Jumper.JumpTo` _returnvalue Destination)))

(fn `UserConstructionScript`)