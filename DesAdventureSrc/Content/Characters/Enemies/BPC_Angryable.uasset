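; Actor component for enemies that tracks whether the owner is angry.
; GetAngry and CalmDown set the IsAngry flag only when its state actually changes, then fire the OnGotAngry or OnCalmedDown dispatcher.
; An Is Angry function exposes the current state to other Blueprints.
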(event `Get Angry`
  (if (not (`self.bIsAngry`))
    (set `self.bIsAngry` true)
    (`self.OnGotAngry`)))

(event `Calm Down`
  (if (`self.bIsAngry`)
    (set `self.bIsAngry` false)
    (`self.OnCalmedDown`)))

(fn `Is Angry`
  (returns (Result :type Boolean))
  (return (`self.bIsAngry`)))